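; Combat manager that populates the battlefield with player and enemy pawns when play begins.
; It resets its tracking arrays and slot counters, then walks every row of DT_CharacterConfig to spawn that row's character class.
; Each spawn takes the next predefined player or enemy position based on the row's player flag, receives its stats through BP_BasePawn's SetStats, and joins the Players or Enemies array.
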(event `self.ReceiveBeginPlay`
  (`self.SetupCombatField`))

(fn `SetupCombatField`
  (`self.ClearShitFromArrays`)
  (bind _outrownames (`DataTableFunctionLibrary.GetDataTableRowNames` "/Game/Blueprints/DT/DT_CharacterConfig.DT_CharacterConfig"))
  (for _array_element _outrownames
    (bind _returnvalue (`|GetDataTableRow` "/Game/Blueprints/DT/DT_CharacterConfig.DT_CharacterConfig" _array_element)
      (:`then`
        (bind _output_get (set `self.CharacterParams` _returnvalue))
        (`self.SpawnEntity` _output_get)))))

(fn `SpawnEntity`
  (params (CharacterParams :type "/Game/Blueprints/Structs/S_CharacterConfig Structure"))
  (bind _s_characterconfig (make `/Game/Blueprints/Structs/S_CharacterConfig` CharacterParams_CharacterClass_19_95CE12464C0E4873343993916713D4CA CharacterParams_bIsPlayer_5_687153FC4D72735A5D738BAE4D825E03 CharacterParams_Health_12_51D6D8714682FFA51B21328D13424CA8 CharacterParams_MaxHealth_11_4AFC97B54DCF5187ACB6209BCBFF0945 CharacterParams_Weakness_15_C3BEDDD24926B39B6D9382856DDCC5B2))
  (if CharacterParams_bIsPlayer_5_687153FC4D72735A5D738BAE4D825E03
    (bind _returnvalue (`|SpawnActorFromClass` CharacterParams_CharacterClass_19_95CE12464C0E4873343993916713D4CA (`KismetMathLibrary.MakeTransform` (`|GetArrayItem` (`self.PlayerSpawnPositions`) (`self.PlayerSpawnsOccupied`))) "Undefined" "MultiplyWithRoot" null null))
    (bind _asbp_base_pawn (cast `/Game/Blueprints/Characters/BP_BasePawn` _returnvalue))
    (`/Game/Blueprints/Characters/BP_BasePawn.SetStats` _asbp_base_pawn _s_characterconfig)
    (`KismetArrayLibrary.Array_Add` (`self.Players`) _asbp_base_pawn)
    (`self.IncrementPlayerSpawnsOccupied`)
    (return)
    (else
      (bind _returnvalue_2 (`|SpawnActorFromClass` CharacterParams_CharacterClass_19_95CE12464C0E4873343993916713D4CA (`KismetMathLibrary.MakeTransform` (`|GetArrayItem` (`self.EnemySpawnPositions`) (`self.EnemySpawnsOccupied`))) "Undefined" "MultiplyWithRoot" null null))
      (bind _asbp_base_pawn_2 (cast `/Game/Blueprints/Characters/BP_BasePawn` _returnvalue_2))
      (`/Game/Blueprints/Characters/BP_BasePawn.SetStats` _asbp_base_pawn_2 _s_characterconfig)
      (`KismetArrayLibrary.Array_Add` (`self.Enemies`) _returnvalue_2)
      (`self.IncrementEnemySpawnsOccupied`)
      (return))))

(fn `UserConstructionScript`)