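; Health component that stores an actor's current health, maximum health and invincibility flag.
; Damage is skipped while invincible, routes negative amounts unnegated to Heal, and calls Die when health minus damage, re-evaluated after subtraction, falls below zero.
; Heal caps health at the maximum, and SetMaxHealth rejects negative values.
; SetHealth sets any positive input to maximum health instead of the given value.
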(fn `Damage`
  (params (DamageToTake :type "Float (double-precision)"))
  (bind _returnvalue (- (`self.CurrentHealth`) DamageToTake))
  (if (`self.bIsInvincible`)
    (return)
    (elif (< DamageToTake 0.0)
      (`self.Heal` DamageToTake)
      (else
        (set `self.CurrentHealth` _returnvalue)
        (if (< _returnvalue 0.0)
          (`self.Die`)
          (return)
          (else
            (return)))))))

(fn `Heal`
  (params (HealthToAdd :type "Float (double-precision)"))
  (bind _returnvalue (+ HealthToAdd (`self.CurrentHealth`)))
  (if (> _returnvalue (`self.MaxHealth`))
    (set `self.CurrentHealth` (`self.MaxHealth`))
    (return)
    (else
      (set `self.CurrentHealth` _returnvalue)
      (return))))

(fn `SetHealth`
  (params (CurrentHealth :type "Float (double-precision)"))
  (if (> CurrentHealth 0.0)
    (set `self.CurrentHealth` (`self.MaxHealth`))
    (return)
    (else
      (set `self.CurrentHealth` CurrentHealth)
      (return))))

(fn `SetInvincibility`
  (params (bIsInvincible :type Boolean))
  (returns (Output_Get :type Boolean))
  (bind _output_get (set `self.bIsInvincible` bIsInvincible))
  (return _output_get))

(fn `SetMaxHealth`
  (params (NewMaxHealth :type "Float (double-precision)"))
  (if (< NewMaxHealth 0.0)
    (return)
    (else
      (set `self.MaxHealth` NewMaxHealth)
      (return))))